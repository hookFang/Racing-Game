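; Coin pickup actor that adds to the player car's coin count when collected.
; Tick spins the Cylinder by a fixed roll step each frame, independent of delta time.
; Any overlap on the Box plays a 2D explosion sound, then casts player pawn 0 to Car_BluePrint without checking the overlapping actor.
; On a successful cast it adds its Coin value to Coins and destroys itself.
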(event OnComponentBeginOverlap(Box)
  (params (OverlappedComponent :type Primitive%20Component%20Object%20Reference) (OtherActor :type Actor%20Object%20Reference) (OtherComp :type Primitive%20Component%20Object%20Reference) (OtherBodyIndex :type Integer) (bFromSweep :type Boolean) (SweepResult :type Hit%20Result%20Structure%20%28by%20ref%29))
  (Audio|PlaySound2D "/Game/StarterContent/Audio/Explosion02.Explosion02" 1.0 1.0 0.0 0 0)
  (bind _ascar_blue_print (Utilities|Casting|CastToCar_BluePrint (Game|Player|GetPlayerPawn 0)))
  (Variables|/Game/Cars/Skeletons/Car_BluePrint.Car_BluePrint_C|Setcoins _ascar_blue_print (+ (Variables|/Game/Cars/Skeletons/Car_BluePrint.Car_BluePrint_C|Getcoins _ascar_blue_print) (Variables|Default|Getcoin)))
  (Actor|DestroyActor))

(event EventTick
  (params (DeltaSeconds :type Float%20%28single-precision%29))
  (bind _cylinder (Variables|Default|GetCylinder))
  (bind _relativerotation (Variables|/Script/Engine.SceneComponent|GetRelativeRotation _cylinder))
  ;[1 1 1] This is for coin rotation
  (Transformation|SetRelativeRotation _cylinder (Math|Rotator|MakeRotator (+ (.roll _relativerotation) 2.0) (.pitch _relativerotation) (.yaw _relativerotation)) false false))

(fn ConstructionScript)