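; RacingGame Blueprint that keeps a running clock in Minutes, Seconds and Milliseconds variables, presumably as the race timer.
; Tick feeds a short Delay that increments Milliseconds, which carries into Seconds after exceeding 100, then into Minutes after Seconds exceeds 60.
; Milliseconds acts as a hundredths counter, but its pace depends on frame rate because it counts Delay completions rather than delta time.
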(event EventTick
  (params (DeltaSeconds :type Float%20%28single-precision%29))
  (Utilities|FlowControl|Delay 0.01)
  (Variables|Default|Setmilliseconds (+ (Variables|Default|Getmilliseconds) 1))
  (if (> (Variables|Default|Getmilliseconds) 100)
    (Variables|Default|Setseconds (+ (Variables|Default|Getseconds) 1))
    (Variables|Default|Setmilliseconds 0)
    (if (> (Variables|Default|Getseconds) 60)
      (Variables|Default|Setminutes (+ 1 (Variables|Default|Getminutes)))
      (Variables|Default|Setseconds 0))))

(fn ConstructionScript)